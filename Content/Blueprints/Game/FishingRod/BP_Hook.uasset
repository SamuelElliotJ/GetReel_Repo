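; BP_Hook is the fishing rod's hook, which starts the minigame when a fish is hooked.
; Init_Hook attaches the end of its cable to the rod's Anchor and stores the rod and game mode references.
; HookEvent passes a one-shot gate, stores the actor as the catch if it is an AI_Fish, then calls PlayMinigame on the BP_Base_Character found by class lookup.
; GetHookRef returns the hook itself.
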(event `Init_Hook`
  (params (FishingRodRef :type "/Game/Blueprints/Game/FishingRod/BP_FishingRod Object Reference") (GameMode :type "/Game/Blueprints/Core/Gamemodes/GM_GetReel_Game Object Reference"))
  (`CableComponent.SetAttachEndToComponent` (`self.Cable`) (`/Game/Blueprints/Game/FishingRod/BP_FishingRod.Anchor` FishingRodRef) "None")
  (set `self.Fishing Rod Ref` FishingRodRef)
  (set `self.Game Mode` GameMode))

(event `/Game/Blueprints/Game/Interface/BPI_Fishing.HookEvent`
  (params (Actor :type "Actor Object Reference"))
  (`/Engine/EditorBlueprintResources/StandardMacros.DoOnce` false
    (:`Completed`
      (bind _asai_fish (cast `/Game/Blueprints/Game/Fish/AI_Fish` Actor))
      (set `self.CaughtActorRef` _asai_fish)
      (bind _returnvalue (`GameplayStatics.GetActorOfClass` "/Game/Blueprints/Characters/BP_Base_Character.BP_Base_Character_C"))
      (`/Game/Blueprints/Characters/BP_Base_Character.Play_Minigame` _returnvalue))))

(fn `Get_HookRef`
  (returns (TargetRef :type "Actor Object Reference"))
  (return self))

(fn `UserConstructionScript`)