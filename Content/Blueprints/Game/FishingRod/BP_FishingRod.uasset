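; BP_FishingRod is the player's fishing rod, turning action presses into casting and catching.
; With no hook out, a press plays the cast montage, whose notify spawns a BP_Hook at the target and hides the rod's hook mesh and cable.
; With a hook out, a DoOnce-gated press resolves any on-screen GameMode minigame, passing the catch to the player or destroying the hook.
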(event `self.ReceiveBeginPlay`
  ;[1 1 1] Bind Events On Begin Play
  (add `/Game/Blueprints/Characters/BP_Base_Character.ActionPressed` (`self.PlayerRef`) (`|CreateDelegate` :!event `ActionPressed`)))

(event `ActionPressed`
  (params (Location :type "Vector Structure"))
  ;[1 1 1] Handle Fishing Mechanics
  (set `self.TargetLoc` Location)
  (`/Engine/EditorBlueprintResources/StandardMacros.IsValid` (`self.HookRef`)
    (:`Is Valid`
      (`/Engine/EditorBlueprintResources/StandardMacros.DoOnce` false :!label _label
        (:`Completed`
          (`self.CatchFish`))))
    (:`Is Not Valid`
      (`self.ThrowLine`)
      (goto _label :!via `Reset`))))

(event `ThrowLine`
  ;[1 1 1] Handle Fishing Mechanics
  (`KismetSystemLibrary.PrintString` "Throw Line")
  (bind _notifyname (`|PlayMontage` (`Character.Mesh` (`self.PlayerRef`)) "/Game/Blueprints/J016221L/Proto_Character/Proto_Animation/Fishing_Cast_Montage.Fishing_Cast_Montage")
    (:`OnNotifyBegin`
      (`KismetSystemLibrary.PrintString` (`KismetStringLibrary.Conv_NameToString` _notifyname))
      (bind _returnvalue (`|SpawnActorFromClass` "/Game/Blueprints/Game/FishingRod/BP_Hook.BP_Hook_C" (`KismetMathLibrary.MakeTransform` (`self.TargetLoc`)) "Undefined" "MultiplyWithRoot" null null))
      (`/Game/Blueprints/Game/FishingRod/BP_Hook.Init_Hook` _returnvalue self (`self.GameMode`))
      (set `self.HookRef` _returnvalue)
      (`SceneComponent.SetHiddenInGame` (`self.SM_Hook`) true false)
      (`SceneComponent.SetHiddenInGame` (`self.Cable`) true false))))

(event `CatchFish`
  (bind _hookref (`self.HookRef`))
  (bind _playerref (`self.PlayerRef`))
  ;[1 1 1] Handle Fishing Mechanics
  (`KismetSystemLibrary.PrintString` "Attempt to Catch Fish")
  (if (`Widget.IsInViewport` (`/Game/Blueprints/Core/Gamemodes/GM_GetReel_Game.Minigame` (`self.GameMode`)))
    (bind _success (`/Game/Widgets/Placeholder/W_Minigame.FishCaught?` (`/Game/Blueprints/Core/Gamemodes/GM_GetReel_Game.Minigame` (`self.GameMode`))))
    (if _success
      (`KismetSystemLibrary.PrintString` "Fish Caught Successfully" true true (struct :`G` 0.66 :`B` 1.0 :`A` 1.0) 10.0)
      (`/Game/Blueprints/Core/Gamemodes/GM_GetReel_Game.End_Minigame` (`self.GameMode`))
      (`/Engine/EditorBlueprintResources/StandardMacros.IsValid` _playerref
        (:`Is Valid`
          (`/Game/Blueprints/Characters/BP_Base_Character.FishCaught` _playerref (`/Game/Blueprints/Game/FishingRod/BP_Hook.CaughtActorRef` _hookref) _hookref)))
      (else
        (`self.K2_DestroyActor` (`self.HookRef`))
        (`KismetSystemLibrary.PrintString` "Fish Got Away" true true (struct :`G` 0.66 :`B` 1.0 :`A` 1.0) 10.0)
        (`/Game/Blueprints/Core/Gamemodes/GM_GetReel_Game.End_Minigame` (`self.GameMode`))))
    (else
      (`self.K2_DestroyActor` (`self.HookRef`)))))

(fn `UserConstructionScript`)