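; Fishing spear projectile that the player aims with the mouse and throws to catch fish, with inventory upgrades for speed and cooldown.
; Holding action runs looping cursor traces that move a crosshair and redden the targeted fish, starting an aim-deviation timer after a delay.
; Release launches via SuggestProjectileVelocity at the fish or crosshair, then triggers the player's spear-count check after cooldown.
; Sphere overlap reports caught fish to the player.
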(event `self.ReceiveBeginPlay`
  (bind _asgm_get_reel_game (cast `/Game/Blueprints/Core/Gamemodes/GM_GetReel_Game` (`GameplayStatics.GetGameMode`)))
  (bind _output_get (set `self.GameMode` _asgm_get_reel_game))
  (bind _inventory_items (`/Game/Blueprints/Core/GameInstance/BP_GI_GetReel.Func_GetInventoryItems` (`/Game/Blueprints/Core/Gamemodes/GM_GetReel_Game.GameInstance` _output_get)))
  (if (`KismetArrayLibrary.Array_Contains` _inventory_items "/Game/Blueprints/Game/DataAssets/ShopItems/Upgrades/Bronze/DA_Upgrade_Bronze_Spear_Speed.DA_Upgrade_Bronze_Spear_Speed")
    (set `self.Launch Speed` 4000.0))
  (if (`KismetArrayLibrary.Array_Contains` _inventory_items "/Game/Blueprints/Game/DataAssets/ShopItems/Upgrades/Bronze/DA_Upgrade_Bronze_Spear_Cooldown.DA_Upgrade_Bronze_Spear_Cooldown")
    (set `self.CoolDown` 1.0)))

(event `LineTraceFish`
  (bind (_worldlocation _worlddirection) (`PlayerController.DeprojectMousePositionToWorld` (`GameplayStatics.GetPlayerController` 0)))
  (bind _outactors (`GameplayStatics.GetAllActorsOfClass` "/Game/Blueprints/Game/Fish/AI_Fish_Active.AI_Fish_Active_C"))
  (for _array_element _outactors
    (`/Game/Blueprints/Game/Fish/AI_Fish_Active.SetColour` _array_element (struct :`R` 0.070588 :`G` 0.070588 :`B` 0.070588 :`A` 1.0)))
  (bind (_outhit _returnvalue) (`KismetSystemLibrary.LineTraceSingleForObjects` _worldlocation (+ _worldlocation (* _worlddirection 10000.0) (`self.RandomDeviation`)) (`|MakeArray` "ObjectTypeQuery5" :!type "EObjectTypeQuery Enum")))
  (if _returnvalue
    (bind _asai_fish_active (cast `/Game/Blueprints/Game/Fish/AI_Fish_Active` (`.HitActor` (`GameplayStatics.BreakHitResult` _outhit))))
    (set `self.AimedFish` _asai_fish_active)
    (`/Game/Blueprints/Game/Fish/AI_Fish_Active.SetColour` _asai_fish_active (struct :`R` 1.0 :`A` 1.0))))

(event `/Game/Blueprints/Game/FishingRod/BPI_FishingRef.SendRefs`
  (params (PlayerRef :type "/Game/Blueprints/Characters/BP_Base_Character Object Reference") (GameMode :type "/Game/Blueprints/Core/Gamemodes/GM_GetReel_Game Object Reference"))
  (bind _playerref (`self.PlayerRef`))
  (set `self.PlayerRef` PlayerRef)
  (set `self.GameMode` GameMode)
  (add `/Game/Blueprints/Characters/BP_Base_Character.ActionPressed` _playerref (`|CreateDelegate` :!event `ActionPressed`))
  (add `/Game/Blueprints/Characters/BP_Base_Character.ActionReleased` _playerref (`|CreateDelegate` :!event `ActionReleased`)))

(event `ActionPressed`
  (`/Engine/EditorBlueprintResources/StandardMacros.DoOnce` false
    (:`Completed`
      (set `self.RandomDeviation` (0.0 0.0 0.0))
      (`self.PlotTrajectory`)
      (bind _returnvalue (`KismetSystemLibrary.K2_SetTimerDelegate` (delegate `PlotTrajectory`) 0.01 true))
      (set `self.HeldTimer` _returnvalue)
      (`KismetSystemLibrary.K2_SetTimerDelegate` (delegate `StartDeviating`) 3.0)
      (`GameplayStatics.PlaySound2D` "/Game/Blueprints/BGM_SE/FishingMechRelated/MS_ThrowSpear.MS_ThrowSpear" 1.0 1.0 0.0 null null))))

(event `StartDeviating`
  (bind _returnvalue (`KismetSystemLibrary.K2_SetTimerDelegate` (`|CreateDelegate` :!event `Deviation`) 0.01 true))
  (set `self.DeviationTimer` _returnvalue))

(event `PlotTrajectory`
  (`self.LineTraceFish`)
  (bind _location (`self.LineTrace_Cursor`))
  (`self.Crosshair`
    (:`then`
      _)
    (:`else`
      (`self.SpawnCrosshair` (`KismetMathLibrary.Conv_VectorToTransform` _location))))
  (`self.K2_SetActorLocation` (`self.Crosshair`) _location false true))

(event `SpawnCrosshair`
  (params (SpawnTransform :type "Transform Structure"))
  (bind _returnvalue (`|SpawnActorFromClass` "/Game/Blueprints/Game/FishingRod/BP_Crosshair.BP_Crosshair_C" SpawnTransform "Undefined" "MultiplyWithRoot" null null))
  (set `self.Crosshair` _returnvalue))

(event `ActionReleased`
  (bind _returnvalue (`self.K2_GetActorLocation`))
  (bind _launch_speed (`self.Launch Speed`))
  (bind _projectilemovement (`self.ProjectileMovement`))
  (bind _aimedfish (`self.AimedFish`))
  (bind _projectilemovement_2 (`self.ProjectileMovement`))
  (`/Engine/EditorBlueprintResources/StandardMacros.DoOnce` false
    (:`Completed`
      (`KismetSystemLibrary.K2_ClearAndInvalidateTimerHandle` (`self.HeldTimer`))
      (`KismetSystemLibrary.K2_ClearAndInvalidateTimerHandle` (`self.DeviationTimer`))
      (bind _outactors (`GameplayStatics.GetAllActorsOfClass` "/Game/Blueprints/Game/Fish/AI_Fish_Active.AI_Fish_Active_C"))
      (for _array_element _outactors
        (`/Game/Blueprints/Game/Fish/AI_Fish_Active.SetColour` _array_element (struct :`R` 0.070588 :`G` 0.070588 :`B` 0.070588 :`A` 1.0)))
      (`/Engine/EditorBlueprintResources/StandardMacros.IsValid` (`self.Crosshair`)
        (:`Is Valid`
          (`/Engine/EditorBlueprintResources/StandardMacros.IsValid` _aimedfish
            (:`Is Valid`
              (bind (_tossvelocity _returnvalue_2) (`GameplayStatics.BlueprintSuggestProjectileVelocity` _returnvalue (`self.K2_GetActorLocation` _aimedfish) _launch_speed 0.0 "DoNotTrace"))
              (if _returnvalue_2
                (set `MovementComponent.Velocity` _tossvelocity _projectilemovement_2))
              (`ActorComponent.Activate` _projectilemovement_2 false))
            (:`Is Not Valid`
              (bind (_tossvelocity_2 _returnvalue_3) (`GameplayStatics.BlueprintSuggestProjectileVelocity` _returnvalue (`self.K2_GetActorLocation` (`self.Crosshair`)) _launch_speed 0.0 "DoNotTrace"))
              (if _returnvalue_3
                (set `MovementComponent.Velocity` _tossvelocity_2 _projectilemovement))
              (`ActorComponent.Activate` _projectilemovement false)))
          (`self.K2_DestroyActor` (`self.Crosshair`))
          (`KismetSystemLibrary.Delay` (`self.CoolDown`))
          (`/Game/Blueprints/Characters/BP_Base_Character.Check_SpearCount` (`self.PlayerRef`) true))
        (:`Is Not Valid`
          (`/Game/Blueprints/Characters/BP_Base_Character.Check_SpearCount` (`self.PlayerRef`) false))))))

(event `self.Sphere.OnComponentBeginOverlap`
  (params (OverlappedComponent :type "PrimitiveComponent Object Reference") (OtherActor :type "Actor Object Reference") (OtherComp :type "PrimitiveComponent Object Reference") (OtherBodyIndex :type Integer) (bFromSweep :type Boolean) (SweepResult :type "HitResult Structure (by ref)"))
  (bind _asai_fish_active (cast `/Game/Blueprints/Game/Fish/AI_Fish_Active` OtherActor))
  (`/Game/Blueprints/Characters/BP_Base_Character.FishCaught` (`self.PlayerRef`) _asai_fish_active null false))

(event `Deviation`
  (set `self.RandomDeviation` (`self.RandomDeviation`)))

(fn `LineTrace_Cursor`
  (returns (Location :type "Vector Structure"))
  (bind (_worldlocation _worlddirection) (`PlayerController.DeprojectMousePositionToWorld` (`GameplayStatics.GetPlayerController` 0)))
  (bind (_outhit _returnvalue) (`KismetSystemLibrary.LineTraceSingleForObjects` _worldlocation (+ _worldlocation (* _worlddirection 10000.0) (`self.RandomDeviation`)) (`|MakeArray` "ObjectTypeQuery1" :!type "EObjectTypeQuery Enum")))
  (if _returnvalue
    (return (`.Location` (`GameplayStatics.BreakHitResult` _outhit)))))

(fn `UserConstructionScript`)