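; Main menu game mode for GetReel that builds the menu widget switcher and drives save loading and character selection.
; On BeginPlay it creates the menu, passes the GameInstance's save-exists check to the Load Game toggle, and binds load and swap events.
; Loading a slot goes through the GameInstance, then changes scene to the ocean dock.
; Swap events cycle a wrapping index across three meshes on the level's BP_CharacterSelecter.
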(event `self.ReceiveBeginPlay`
  (bind _asbp_gi_get_reel (cast `/Game/Blueprints/Core/GameInstance/BP_GI_GetReel` (`GameplayStatics.GetGameInstance`)))
  (set `self.GameInstance` _asbp_gi_get_reel)
  (`self.Init_Widget`)
  (bind _returnvalue (`GameplayStatics.GetActorOfClass` "/Game/Blueprints/Game/BP_CharacterSelecter.BP_CharacterSelecter_C"))
  (bind _output_get (set `self.CharacterSelector` _returnvalue))
  (`/Game/Blueprints/Game/BP_CharacterSelecter.SetCharacterMesh` _output_get (`self.Index`)))

(event `Init_Widget`
  (bind _returnvalue (`|CreateWidget` "/Game/Blueprints/Widgets/BaseWidgets/W_Placeholder_WidgetSwitcher.W_Placeholder_WidgetSwitcher_C"))
  (bind _output_get (set `self.W_MainMenu` _returnvalue))
  (bind _savegameexists_ (`/Game/Blueprints/Core/GameInstance/BP_GI_GetReel.Func_DoesASaveGameExist` (`self.GameInstance`)))
  (`/Game/Blueprints/Widgets/BaseWidgets/W_Placeholder_WidgetSwitcher.Disable_LoadGame` _output_get _savegameexists_)
  (`UserWidget.AddToViewport` _output_get 0)
  (add `/Game/Blueprints/Widgets/Placeholder/OnHold/W_Placeholder_LoadGame.LoadGameFromSlot` (`/Game/Blueprints/Widgets/BaseWidgets/W_Placeholder_WidgetSwitcher.W_Placeholder_LoadGame` _output_get) (`|CreateDelegate` :!event `LoadGameFromSlot`))
  (bind _w_placeholder_characterselect (`/Game/Blueprints/Widgets/BaseWidgets/W_Placeholder_WidgetSwitcher.W_Placeholder_CharacterSelect` _output_get))
  (add `/Game/Blueprints/Widgets/SubWidgets/W_Placeholder_CharacterSelect.SwapCharacter_Left` _w_placeholder_characterselect (`|CreateDelegate` :!event `SwapCharacter_Left`))
  (add `/Game/Blueprints/Widgets/SubWidgets/W_Placeholder_CharacterSelect.SwapCharacter_Right` _w_placeholder_characterselect (`|CreateDelegate` :!event `SwapCharacter_Right`)))

(event `LoadGameFromSlot`
  (params (Slot :type Integer))
  (bind _gameinstance (`self.GameInstance`))
  (`/Game/Blueprints/Core/GameInstance/BP_GI_GetReel.Func_LoadGameFromSlot` _gameinstance Slot)
  (`/Game/Blueprints/Core/GameInstance/BP_GI_GetReel.ChangeScene` _gameinstance "/Game/Levels/L_Ocean_Dock.L_Ocean_Dock"))

(event `SwapCharacter_Left`
  (`/Engine/EditorBlueprintResources/StandardMacros.DecrementInt` (`self.Index`)
    (:`  `
      (if (< (`self.Index`) 0)
        (bind _output_get (set `self.Index` 2))
        (`/Game/Blueprints/Game/BP_CharacterSelecter.SetCharacterMesh` (`self.CharacterSelector`) _output_get)
        (else
          (`/Game/Blueprints/Game/BP_CharacterSelecter.SetCharacterMesh` (`self.CharacterSelector`) (`self.Index`)))))))

(event `SwapCharacter_Right`
  (`/Engine/EditorBlueprintResources/StandardMacros.IncrementInt` (`self.Index`)
    (:`  `
      (if (> (`self.Index`) 2)
        (set `self.Index` 0)
        (`/Game/Blueprints/Game/BP_CharacterSelecter.SetCharacterMesh` (`self.CharacterSelector`) 0)
        (else
          (`/Game/Blueprints/Game/BP_CharacterSelecter.SetCharacterMesh` (`self.CharacterSelector`) (`self.Index`)))))))

(fn `UserConstructionScript`)