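; Game mode for GetReel, a fishing game, that runs the day loop across the ocean and shop levels.
; BeginPlay loads saved progress from the game instance, then either sets up ocean play (day count, raised quota, HUD, player, minigame, day/night cycle) or shows the shop widget.
; Catches add money and unique fish types; day start and end quick-save, and day end opens the shop.
; Pausing sets global time dilation to zero.
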(event `Init_ShopHUD`
  (bind _returnvalue (`|CreateWidget` "/Game/Blueprints/Widgets/Placeholder/W_Placeholder_Shop.W_Placeholder_Shop_C"))
  (bind _output_get (set `self.ShopHUD` _returnvalue))
  (`/Game/Blueprints/Widgets/Placeholder/W_Placeholder_Shop.Func_SetInfo` _output_get (`self.GameInstance`))
  (`UserWidget.AddToViewport` _output_get 0))

(event `self.ReceiveBeginPlay`
  (`self.Init_GameInstance`)
  (bind _returnvalue (`GameplayStatics.GetCurrentLevelName` true))
  (switch `string` _returnvalue
    (:`L_DemoOcean`
      (`self.IncrementDay`)
      (`self.Init_Quota`)
      (`self.Init_PlayerHUD`)
      (`self.Init_Player`)
      (`self.Init_DayNight`))
    (:`L_Shop`
      (`self.Init_ShopHUD`))))

(event `Init_GameInstance`
  (bind _asbp_gi_get_reel (cast `/Game/Blueprints/Core/GameInstance/BP_GI_GetReel` (`GameplayStatics.GetGameInstance`)))
  (bind _output_get (set `self.GameInstance` _asbp_gi_get_reel))
  (bind (_saved_daycount _saved_money _saved_quota _caughtfishtypes) (`/Game/Blueprints/Core/GameInstance/BP_GI_GetReel.Func_GetSavedVar` _output_get))
  (set `self.DayCount[TBD]` _saved_daycount)
  (set `self.Money[TBD]` _saved_money)
  (set `self.Quota[TBD]` _saved_quota)
  (set `self.CaughtFishTypes` _caughtfishtypes))

(event `IncrementDay`
  (`/Engine/EditorBlueprintResources/StandardMacros.IncrementInt` (`self.DayCount[TBD]`)))

(event `Init_PlayerHUD`
  (bind _returnvalue (`|CreateWidget` "/Game/Blueprints/Widgets/Placeholder/W_Placeholder_Game.W_Placeholder_Game_C" null self))
  (bind _output_get (set `self.GameHUD` _returnvalue))
  (`/Game/Blueprints/Widgets/Placeholder/W_Placeholder_Game.Init_HUD` _output_get)
  (`UserWidget.AddToViewport` _output_get 0)
  (add `/Game/Blueprints/Widgets/Placeholder/W_Placeholder_Day.SwitchWidget` (`/Game/Blueprints/Widgets/Placeholder/W_Placeholder_Game.W_Placeholder_Day` _output_get) (`|CreateDelegate` :!event `Start_Game`))
  (add `Button.OnClicked` (`/Game/Blueprints/Widgets/Placeholder/W_Placeholder_PauseMenu.BTN_Continue` (`/Game/Blueprints/Widgets/Placeholder/W_Placeholder_Game.W_Placeholder_PauseMenu` (`self.GameHUD`))) (`|CreateDelegate` :!event `PauseGame`)))

(event `Init_Player`
  (bind _returnvalue (`GameplayStatics.GetActorOfClass` "/Game/Blueprints/Core/PlayerController/PC_GetReel.PC_GetReel_C"))
  (bind _output_get (set `self.PlayerController` _returnvalue))
  (`/Game/Blueprints/Core/PlayerController/PC_GetReel.Func_SpawnPlayer` _output_get)
  (`/Game/Blueprints/Core/PlayerController/PC_GetReel.Func_DisablePlayer` _output_get true)
  (`/Game/Blueprints/Core/PlayerController/PC_GetReel.Func_SpawnMinigame` _output_get self)
  (add `/Game/Blueprints/Core/PlayerController/PC_GetReel.SetGamePaused` _output_get (`|CreateDelegate` :!event `PauseGame`)))

(event `Init_DayNight`
  (bind _returnvalue (`GameplayStatics.GetActorOfClass` "/Game/Blueprints/WillCook/BP_DayNight.BP_DayNight_C"))
  (bind _output_get (set `self.DayNight_Ref` _returnvalue))
  (add `/Game/Blueprints/WillCook/BP_DayNight.DayFinished` _output_get (`|CreateDelegate` :!event `DayFinished`)))

(event `Init_Quota`
  (set `self.Quota[TBD]` (* (`self.Quota[TBD]`) 1.15)))

(event `Start_Game`
  (`/Engine/EditorBlueprintResources/StandardMacros.DoOnce` false
    (:`Completed`
      (`/Game/Blueprints/WillCook/BP_DayNight.Start_Day` (`self.DayNight_Ref`))
      (`/Game/Blueprints/Widgets/Placeholder/W_Placeholder_Game.Update_Day` (`self.GameHUD`) (`self.DayCount[TBD]`))
      (`/Game/Blueprints/Widgets/Placeholder/W_Placeholder_Game.Update_Quota` (`self.GameHUD`) (`self.Quota[TBD]`))
      (`/Game/Blueprints/Widgets/Placeholder/W_Placeholder_Game.Update_Money` (`self.GameHUD`) (`self.Money[TBD]`))
      (`/Game/Blueprints/Core/PlayerController/PC_GetReel.Func_DisablePlayer` (`self.PlayerController`) false)
      (`/Game/Blueprints/Core/GameInstance/BP_GI_GetReel.QuickSave` (`self.GameInstance`) (`self.DayCount[TBD]`) (`self.Money[TBD]`) (`self.Quota[TBD]`) (`self.CaughtFishTypes`) (`/Game/Blueprints/Characters/BP_Base_Character.DisplayName` (`/Game/Blueprints/Core/PlayerController/PC_GetReel.Player Ref` (`self.PlayerController`)))))))

(event `UpdateHUD`
  (params (Data :type "DataAsset_Fish Object Reference"))
  (`/Game/Blueprints/Widgets/Placeholder/W_Placeholder_GameHUD.AddFishInfo` (`/Game/Blueprints/Widgets/Placeholder/W_Placeholder_Game.W_Placeholder_GameHUD` (`self.GameHUD`)) Data)
  (bind _output_get (set `self.Money[TBD]` (+ (`self.Money[TBD]`) (`DataAsset_Fish.AssetValue` Data))))
  (`/Game/Blueprints/Widgets/Placeholder/W_Placeholder_Game.Update_Money` (`self.GameHUD`) _output_get))

(event `DayFinished`
  (`/Game/Blueprints/Core/GameInstance/BP_GI_GetReel.QuickSave` (`self.GameInstance`) (`self.DayCount[TBD]`) (`self.Money[TBD]`) (`self.Quota[TBD]`) (`self.CaughtFishTypes`) (`/Game/Blueprints/Characters/BP_Base_Character.DisplayName` (`/Game/Blueprints/Core/PlayerController/PC_GetReel.Player Ref` (`self.PlayerController`))))
  (`GameplayStatics.OpenLevelBySoftObjectPtr` "/Game/Levels/L_Shop.L_Shop"))

(event `PauseGame`
  (bind _canpause_ (`/Game/Blueprints/Widgets/Placeholder/W_Placeholder_Game.Func_CanPause` (`self.GameHUD`)))
  (if _canpause_
    (if (`self.Paused?`)
      (`/Game/Blueprints/Widgets/Placeholder/W_Placeholder_Game.ClosePauseMenu` (`self.GameHUD`))
      (set `self.Paused?` false)
      (`GameplayStatics.SetGlobalTimeDilation` 1.0)
      (else
        (`/Game/Blueprints/Widgets/Placeholder/W_Placeholder_Game.OpenPauseMenu` (`self.GameHUD`))
        (set `self.Paused?` true)
        (`GameplayStatics.SetGlobalTimeDilation` 0.0)))))

(event `Update_FishCaught`
  (params (DataAsset :type "DataAsset_Fish Object Reference"))
  (`KismetArrayLibrary.Array_AddUnique` (`self.CaughtFishTypes`) DataAsset))

(fn `UserConstructionScript`)