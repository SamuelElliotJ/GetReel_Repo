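; Save game object that holds run progress for what appears to be a fishing game: player class, day count, money, quota and caught fish types.
; One setter function writes all five variables at once and one getter returns them together.
; It only stores data, with no disk save or load logic and no validation in these functions.
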(fn `Func_GetSaveVar`
  (returns (PlayerClass :type "/Game/Blueprints/Characters/BP_Base_Character Class Reference") (DayCount :type Integer) (Money :type "Float (double-precision)") (Quota :type "Float (double-precision)") (CaughtFishTypes :type "Array of DataAsset_Fish Object Reference"))
  (return (`self.PlayerClass`) (`self.DayCount`) (`self.Money`) (`self.Quota`) (`self.CaughtFishTypes`)))

(fn `Func_SetSaveVar`
  (params (PlayerClass :type "/Game/Blueprints/Characters/BP_Base_Character Class Reference") (DayCount :type Integer) (Money :type "Float (double-precision)") (Quota :type "Float (double-precision)") (CaughtFishTypes :type "Array of DataAsset_Fish Object Reference"))
  (set `self.PlayerClass` PlayerClass)
  (set `self.DayCount` DayCount)
  (set `self.Money` Money)
  (set `self.Quota` Quota)
  (set `self.CaughtFishTypes` CaughtFishTypes))