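; PC_GetReel is the player controller for GetReel, handling input setup and the spawning and possession of the player character.
; BeginPlay adds the IMC_GetReel Enhanced Input mapping context.
; Func_SpawnPlayer has BP_PlayerSpawn spawn the game instance's chosen character, falling back to BP_Human_Character, then possesses it.
; Func_DisablePlayer toggles that character's input, while Func_SpawnMinigame is an unfinished stub with disconnected screen-to-world spawn nodes.
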(event `self.ReceiveBeginPlay`
  (bind _returnvalue (pcsubsystem `EnhancedInputLocalPlayerSubsystem` self))
  (`/Engine/EditorBlueprintResources/StandardMacros.IsValid` _returnvalue
    (:`Is Valid`
      (`EnhancedInputSubsystemInterface.AddMappingContext` _returnvalue "/Game/Blueprints/Characters/Input/IMC_GetReel.IMC_GetReel" 0 (struct)))))

(fn `Func_DisablePlayer`
  (params (`Disable?` :type Boolean))
  (bind _player_ref (`self.Player Ref`))
  (if `Disable?`
    (`self.DisableInput` _player_ref self)
    (else
      (`self.EnableInput` _player_ref self))))

(fn `Func_SpawnMinigame`
  (params (GameMode :type "/Game/Blueprints/Core/Gamemodes/GM_GetReel_Game Object Reference")))

(fn `Func_SpawnPlayer`
  (bind _playercharacter (`/Game/Blueprints/Core/GameInstance/BP_GI_GetReel.PlayerCharacter` (`self.GameInstance`)))
  (bind _asbp_gi_get_reel (cast `/Game/Blueprints/Core/GameInstance/BP_GI_GetReel` (`GameplayStatics.GetGameInstance`)))
  (set `self.GameInstance` _asbp_gi_get_reel)
  (bind _returnvalue (`GameplayStatics.GetActorOfClass` "/Game/Blueprints/Game/BP_PlayerSpawn.BP_PlayerSpawn_C"))
  (if (`KismetSystemLibrary.IsValidClass` _playercharacter)
    (bind _playerref (`/Game/Blueprints/Game/BP_PlayerSpawn.Func_SpawnCharacter` _returnvalue _playercharacter))
    (bind _output_get (set `self.Player Ref` _playerref))
    (`self.Possess` _output_get)
    (return)
    (else
      (bind _playerref_2 (`/Game/Blueprints/Game/BP_PlayerSpawn.Func_SpawnCharacter` _returnvalue "/Game/Blueprints/Characters/BP_Human_Character.BP_Human_Character_C"))
      (bind _output_get_2 (set `self.Player Ref` _playerref_2))
      (`self.Possess` _output_get_2)
      (return))))

(fn `UserConstructionScript`)