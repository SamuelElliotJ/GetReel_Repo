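; Game instance for a fishing game that carries player, day, money, quota, caught fish and inventory state and handles saving.
; Events cache that state, open levels, or reset progress except inventory for a new game in L_DemoOcean.
; Functions copy the cache to and from BP_SaveGame in numbered slots, though loading does not restore inventory.
; The save-exists check loops over three slots but returns false as soon as one is missing.
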(event `SetPlayer`
  (params (PlayerCharacter :type "/Game/Blueprints/Characters/BP_Base_Character Class Reference"))
  (set `self.PlayerCharacter` PlayerCharacter))

(event `ChangeScene`
  (params (Level :type "World Soft Object Reference"))
  (`GameplayStatics.OpenLevelBySoftObjectPtr` Level))

(event `QuickSave`
  (params (Saved_DayCount :type Integer) (Saved_Money :type "Float (double-precision)") (Saved_Quota :type "Float (double-precision)") (CaughtFishTypes :type "Array of DataAsset_Fish Object Reference") (`Display Name` :type Name))
  (set `self.Saved_DayCount` Saved_DayCount)
  (set `self.Saved_Money` Saved_Money)
  (set `self.Saved_Quota` Saved_Quota)
  (set `self.CaughtFishTypes` CaughtFishTypes)
  (set `self.Display Name` `Display Name`))

(event `NewGame`
  (set `self.Saved_DayCount` 0)
  (set `self.Saved_Money` 0.0)
  (set `self.Saved_Quota` 1000.0)
  (`KismetArrayLibrary.Array_Clear` (`self.CaughtFishTypes`))
  (`self.ChangeScene` "/Game/Levels/L_DemoOcean.L_DemoOcean"))

(event `AddInventoryItems`
  (params (InventoryItems :type "Array of DataAsset_ShopItem Object Reference"))
  (set `self.Inventory Items` InventoryItems))

(fn `Func_DoesASaveGameExist`
  (returns (`SaveGameExists?` :type Boolean))
  (for _index (range 3)
    (bind _returnvalue (`GameplayStatics.DoesSaveGameExist` (`KismetStringLibrary.Conv_IntToString` _index)))
    (if _returnvalue
      (break)
      (else
        (return false))))
  (return true))

(fn `Func_GetSavedVar`
  (returns (Saved_DayCount :type Integer) (Saved_Money :type "Float (double-precision)") (Saved_Quota :type "Float (double-precision)") (CaughtFishTypes :type "Array of DataAsset_Fish Object Reference") (`Display Name` :type Name) (`Inventory Items` :type "Array of DataAsset_ShopItem Object Reference"))
  (return (`self.Saved_DayCount`) (`self.Saved_Money`) (`self.Saved_Quota`) (`self.CaughtFishTypes`) (`self.Display Name`) (`self.Inventory Items`)))

(fn `Func_LoadGameFromSlot`
  (params (Slot :type Integer))
  (bind _returnvalue (`GameplayStatics.LoadGameFromSlot` (`KismetStringLibrary.Conv_IntToString` Slot)))
  (bind _asbp_save_game (cast `/Game/Blueprints/Core/SaveGame/BP_SaveGame` _returnvalue))
  (set `self.PlayerCharacter` (`/Game/Blueprints/Core/SaveGame/BP_SaveGame.PlayerClass` _asbp_save_game))
  (set `self.Saved_DayCount` (`/Game/Blueprints/Core/SaveGame/BP_SaveGame.DayCount` _asbp_save_game))
  (set `self.Saved_Money` (`/Game/Blueprints/Core/SaveGame/BP_SaveGame.Money` _asbp_save_game))
  (set `self.Saved_Quota` (`/Game/Blueprints/Core/SaveGame/BP_SaveGame.Quota` _asbp_save_game))
  (set `self.CaughtFishTypes` (`/Game/Blueprints/Core/SaveGame/BP_SaveGame.CaughtFishTypes` _asbp_save_game))
  (set `self.Display Name` (`/Game/Blueprints/Core/SaveGame/BP_SaveGame.DisplayName` _asbp_save_game)))

(fn `Func_SaveGameToSlot`
  (params (Slot :type Integer))
  (returns (`Save Successful?` :type Boolean))
  (bind _returnvalue (`GameplayStatics.DoesSaveGameExist` (`KismetStringLibrary.Conv_IntToString` Slot)))
  (if _returnvalue
    (`KismetSystemLibrary.PrintString` "Overwriting Save Slot"))
  (bind _returnvalue_2 (`GameplayStatics.CreateSaveGameObject` "/Game/Blueprints/Core/SaveGame/BP_SaveGame.BP_SaveGame_C"))
  (`/Game/Blueprints/Core/SaveGame/BP_SaveGame.Func_SetSaveVar` _returnvalue_2 (`self.PlayerCharacter`) (`self.Saved_DayCount`) (`self.Saved_Money`) (`self.Saved_Quota`) (`self.CaughtFishTypes`) (`self.Display Name`) (`self.Inventory Items`))
  (bind _returnvalue_3 (`GameplayStatics.SaveGameToSlot` _returnvalue_2 (`KismetStringLibrary.Conv_IntToString` Slot)))
  (if _returnvalue_3
    (`KismetSystemLibrary.PrintString` "Save Successful")
    (return true)
    (else
      (`KismetSystemLibrary.PrintString` "Save UnSuccessful")
      (return false))))