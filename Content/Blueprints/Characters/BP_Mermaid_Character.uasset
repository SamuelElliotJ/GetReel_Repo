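; BP_Mermaid_Character is a mermaid character that creates the player HUD on BeginPlay and throws spears on left click.
; A click traces under the cursor to set the target and flashes a debug sphere there.
; After a short delay, it spawns a Spear above and beside the character, facing that target, and calls its Launcher.
; A DoOnce, reset through the NewSpear event after launch, blocks overlapping throws.
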(event `self.ReceiveBeginPlay`
  ;[1 1 1] Initilise Widget and Player HUD - BeginPlay
  (bind _returnvalue (`|CreateWidget` "/Game/Blueprints/J016221L/Proto_Widgets/W_PlayerHUD.W_PlayerHUD_C"))
  (`UserWidget.AddToViewport` _returnvalue 0))

(event `Key|LeftMouseButton`
  (params (Key :type "Key Structure"))
  (bind _returnvalue (+ (`self.K2_GetActorLocation`) (0.0 30.0 60.0)))
  ;[1 1 1] Spear Throw
  (:`Pressed`
    (`/Engine/EditorBlueprintResources/StandardMacros.DoOnce` false :!label _label
      (:`Completed`
        (bind _output_get (set `self.Set target` (`.Location` (`GameplayStatics.BreakHitResult` (`PlayerController.GetHitResultUnderCursorByChannel` (`GameplayStatics.GetPlayerController` 0) "TraceTypeQuery1" true)))))
        (`KismetSystemLibrary.DrawDebugSphere` _output_get 25.0 12 (struct :`R` 0.027672 :`G` 1.0 :`B` 0.920325 :`A` 1.0) 0.2)
        (`KismetSystemLibrary.Delay` 2.0)
        (bind _returnvalue_2 (`|SpawnActorFromClass` "/Game/Blueprints/R029453M/Spear.Spear_C" (`KismetMathLibrary.MakeTransform` _returnvalue (`KismetMathLibrary.FindLookAtRotation` _returnvalue (`self.Set target`))) "Undefined" "MultiplyWithRoot" null null))
        (`/Game/Blueprints/R029453M/Spear.Launcher` _returnvalue_2 _returnvalue (`self.Set target`))
        (`self.new spear`)))))

(event `new spear`
  ;[1 1 1] Spear Throw
  (goto _label :!via `Reset`))

(fn `UserConstructionScript`
  (`parent.UserConstructionScript`))