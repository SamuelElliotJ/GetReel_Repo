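; Base player character for a fishing game that manages equipped gear, inventory and catches.
; BeginPlay loads GameInstance inventory, creates the minigame widget, equips the rod and spawns any owned net.
; Keys 1 and 2 swap rod and spear, each DoOnce reset by the other, while action input fires dispatchers for gear.
; Catches update GameMode and HUD and drop ragdoll fish into the basket; spears are consumed and nets can randomly break.
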(event `self.ReceiveBeginPlay`
  ;[1 1 1] Begin Play
  (bind _asgm_get_reel_game (cast `/Game/Blueprints/Core/Gamemodes/GM_GetReel_Game` (`GameplayStatics.GetGameMode`)))
  (bind _output_get (set `self.GameMode` _asgm_get_reel_game))
  (`self.AddInventoryItems` (`/Game/Blueprints/Core/GameInstance/BP_GI_GetReel.Inventory Items` (`/Game/Blueprints/Core/Gamemodes/GM_GetReel_Game.GameInstance` _output_get)))
  (bind _returnvalue (`|CreateWidget` "/Game/Blueprints/Widgets/Placeholder/W_Minigame.W_Minigame_C"))
  (set `self.W_Minigame` _returnvalue)
  (`self.Equip_FishingEquipment` "/Game/Blueprints/Game/FishingRod/BP_FishingRod.BP_FishingRod_C")
  (`self.SpawnNet`))

(event `new spear`
  (bind _returnvalue (+ (`self.K2_GetActorLocation`) (0.0 30.0 60.0)))
  ;[1 1 1] Deprecated
  (`/Engine/EditorBlueprintResources/StandardMacros.DoOnce` false :!via `Reset`
    (:`Completed`
      (bind _output_get (set `self.Set target` (`.Location` (`GameplayStatics.BreakHitResult` (`PlayerController.GetHitResultUnderCursorByChannel` (`GameplayStatics.GetPlayerController` 0) "TraceTypeQuery1" true)))))
      (`KismetSystemLibrary.DrawDebugSphere` _output_get 25.0 12 (struct :`R` 0.027672 :`G` 1.0 :`B` 0.920325 :`A` 1.0) 0.2)
      (bind _returnvalue_2 (`|SpawnActorFromClass` "/Game/Blueprints/R029453M/BP_Spear.BP_Spear_C" (`KismetMathLibrary.MakeTransform` _returnvalue (`KismetMathLibrary.FindLookAtRotation` _returnvalue (`self.Set target`))) "Undefined" "MultiplyWithRoot" null self null))
      (`/Game/Blueprints/R029453M/BP_Spear.Launcher` _returnvalue_2 _returnvalue (`self.Set target`))
      (`KismetSystemLibrary.Delay` 0.5)
      (`self.new spear`))))

(event `FishCaught`
  (params (CaughtActor :type "/Game/Blueprints/Game/Fish/AI_Fish_Base Object Reference") (HookRef :type "Actor Object Reference"))
  (bind _gamemode (`self.GameMode`))
  (bind _data (`/Game/Blueprints/Game/Fish/AI_Fish_Base.Data` CaughtActor))
  (bind _gamemode_2 (`self.GameMode`))
  (bind _data_2 (`/Game/Blueprints/Game/Fish/AI_Fish_Base.Data` CaughtActor))
  (bind _returnvalue (`SceneComponent.K2_GetComponentLocation` (`self.FishAnchor`)))
  ;[1 1 1] Fish Caught -  Fix: When second fish caught just add money
  (`self.FishCaught?` CaughtActor)
  (bind _caught_actor (`self.Caught Actor`)
    (:`then`
      (`/Game/Blueprints/Core/Gamemodes/GM_GetReel_Game.UpdateHUD` _gamemode_2 _data_2)
      (`/Game/Blueprints/Core/Gamemodes/GM_GetReel_Game.Update_FishCaught` _gamemode_2 _data_2)
      (bind _returnvalue_2 (`GameplayStatics.GetActorOfClass` "/Game/Blueprints/Game/Fish/BP_Basket.BP_Basket_C"))
      (`/Game/Blueprints/Game/Fish/BP_Basket.SpawnRagdollFish` _returnvalue_2 _data_2)
      (`self.K2_DestroyActor` CaughtActor))
    (:`else`
      (set `self.Caught Actor` _caught_actor)
      (`/Game/Blueprints/Game/Fish/AI_Fish_Passive.DisableFish` CaughtActor)
      (`/Game/Blueprints/Game/Fish/AI_Fish_Passive.ResetMaterial` CaughtActor)
      (`self.K2_SetActorLocation` CaughtActor _returnvalue false true)
      (`self.K2_SetActorRotation` CaughtActor (struct :`Roll` 270.0) false)
      (`NiagaraFunctionLibrary.SpawnSystemAtLocation` "/Game/TopDown/Particles/FishCAught.FishCAught" _returnvalue)
      (`/Game/Blueprints/Core/Gamemodes/GM_GetReel_Game.UpdateHUD` _gamemode _data)
      (`/Game/Blueprints/Core/Gamemodes/GM_GetReel_Game.Update_FishCaught` _gamemode _data)
      (`KismetSystemLibrary.Delay` 1.0)
      (bind _returnvalue_3 (`GameplayStatics.GetActorOfClass` "/Game/Blueprints/Game/Fish/BP_Basket.BP_Basket_C"))
      (`/Game/Blueprints/Game/Fish/BP_Basket.SpawnRagdollFish` _returnvalue_3 _data)
      (`self.K2_DestroyActor` CaughtActor)
      (`/Engine/EditorBlueprintResources/StandardMacros.IsValid` HookRef
        (:`Is Valid`
          (`self.K2_DestroyActor` HookRef))))))

(event `AddInventoryItems`
  (params (InventoryItems :type "Array of DataAsset_ShopItem Object Reference"))
  (set `self.Inventory Items` InventoryItems))

(event `Equip_FishingEquipment`
  (params (Class :type "Actor Class Reference"))
  ;[1 1 1] Spawn Fishing Rod
  (bind _equipped_item (`self.Equipped_Item`)
    (:`then`
      (`self.K2_DestroyActor` _equipped_item))
    (:`else`
      _))
  (bind _returnvalue (`|SpawnActorFromClass` Class (`self.GetTransform`) "AdjustIfPossibleButAlwaysSpawn" "MultiplyWithRoot" null null))
  (bind _output_get (set `self.Equipped_Item` _returnvalue))
  (message `/Game/Blueprints/Game/FishingRod/BPI_FishingRef.SendRefs` _output_get self (`self.GameMode`))
  (`self.K2_AttachToComponent` _returnvalue (`self.Mesh`) "RightHandSocket" "SnapToTarget" "SnapToTarget" "SnapToTarget" true))

(event `EnhancedInput|/Game/Blueprints/Characters/Input/ActionMappings/IA_Action`
  (params (ActionValue :type Boolean) (ElapsedSeconds :type "Float (double-precision)") (TriggeredSeconds :type "Float (double-precision)") (InputAction :type "InputAction Object Reference" :default "/Game/Blueprints/Characters/Input/ActionMappings/IA_Action.IA_Action"))
  (:`Started`
    (`self.ActionPressed`))
  (:`Completed`
    (`self.ActionReleased`)))

(event `Key|One`
  (params (Key :type "Key Structure"))
  (:`Pressed`
    (`/Engine/EditorBlueprintResources/StandardMacros.DoOnce` false :!label _label
      (:`Completed`
        (`self.Equip_FishingEquipment` "/Game/Blueprints/Game/FishingRod/BP_FishingRod.BP_FishingRod_C")
        (`self.Reset_Spear`)))))

(event `Reset_FishingRod`
  (goto _label :!via `Reset`))

(event `Play_Minigame`
  (bind _w_minigame (`self.W_Minigame`))
  (if (not (`Widget.IsInViewport` (`self.W_Minigame`)))
    (`UserWidget.AddToViewport` _w_minigame 0)
    (`/Game/Blueprints/Widgets/Placeholder/W_Minigame.Start_Minigame` _w_minigame)))

(event `Key|Two`
  (params (Key :type "Key Structure"))
  (bind _w_minigame (`self.W_Minigame`))
  (:`Pressed`
    (if (`KismetArrayLibrary.Array_Contains` (`self.Inventory Items`) "/Game/Blueprints/Game/DataAssets/ShopItems/Equipment/DA_ThrowingSpear.DA_ThrowingSpear")
      (`/Engine/EditorBlueprintResources/StandardMacros.DoOnce` false :!label _label_2
        (:`Completed`
          (bind _returnvalue (`GameplayStatics.GetActorOfClass` "/Game/Blueprints/Game/FishingRod/BP_Hook.BP_Hook_C"))
          (`self.K2_DestroyActor` _returnvalue)
          (bind _returnvalue_2 (`GameplayStatics.GetActorOfClass` "/Game/Blueprints/Game/Fish/AI_Fish_Passive.AI_Fish_Passive_C"))
          (`self.K2_DestroyActor` _returnvalue_2)
          (if (`Widget.IsInViewport` _w_minigame)
            (`Widget.RemoveFromParent` _w_minigame)
            (else
              (`self.Equip_FishingEquipment` "/Game/Blueprints/Game/FishingRod/BP_FishingSpear.BP_FishingSpear_C")))
          (`self.Reset_FishingRod`))))))

(event `Reset_Spear`
  (goto _label_2 :!via `Reset`))

(event `End_Minigame`
  (`Widget.RemoveFromParent` (`self.W_Minigame`)))

(event `Check_SpearCount`
  (bind _inventory_items (`self.Inventory Items`))
  (`KismetArrayLibrary.Array_Remove` _inventory_items (`KismetArrayLibrary.Array_Find` _inventory_items "/Game/Blueprints/Game/DataAssets/ShopItems/Equipment/DA_ThrowingSpear.DA_ThrowingSpear"))
  (if (`KismetArrayLibrary.Array_Contains` (`self.Inventory Items`) "/Game/Blueprints/Game/DataAssets/ShopItems/Equipment/DA_ThrowingSpear.DA_ThrowingSpear")
    (`self.Equip_FishingEquipment` "/Game/Blueprints/Game/FishingRod/BP_FishingSpear.BP_FishingSpear_C")
    (else
      (`self.Equip_FishingEquipment` "/Game/Blueprints/Game/FishingRod/BP_FishingRod.BP_FishingRod_C"))))

(event `SpawnNet`
  (if (`KismetArrayLibrary.Array_Contains` (`self.Inventory Items`) "/Game/Blueprints/Game/DataAssets/ShopItems/Equipment/DA_FishingNet.DA_FishingNet")
    (bind _returnvalue (`GameplayStatics.GetActorOfClass` "/Game/Blueprints/Game/FishingNet/BP_NetAnchor.BP_NetAnchor_C"))
    (bind _returnvalue_2 (`|SpawnActorFromClass` "/Game/Blueprints/Game/FishingNet/BP_FishingNet.BP_FishingNet_C" (`self.GetTransform` _returnvalue) "Undefined" "MultiplyWithRoot" null null))
    (set `self.FishingNet` _returnvalue_2)))

(fn `BreakNet`
  (bind _inventory_items (`self.Inventory Items`))
  (if (`KismetMathLibrary.RandomBoolWithWeight` 0.1)
    (`self.K2_DestroyActor` (`self.FishingNet`))
    (`KismetArrayLibrary.Array_Remove` _inventory_items (`KismetArrayLibrary.Array_Find` _inventory_items "/Game/Blueprints/Game/DataAssets/ShopItems/Equipment/DA_FishingNet.DA_FishingNet"))))

(fn `UserConstructionScript`)