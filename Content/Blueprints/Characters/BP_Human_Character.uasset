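; BP_Human_Character is a human character Blueprint whose event graph holds a deprecated fishing system, mostly disconnected.
; ResetFishing clears the line and bobber state, and Init_FishWidget creates a W_CaughtFish widget with empty name and zero value, then adds it to the viewport.
; ThrowLine and SetWidgetVisibility are empty events; the old bobber spawn, launch, reel and visibility logic remains as unreachable nodes.
; The construction script only calls its parent.
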(event `Key|LeftMouseButton`
  (params (Key :type "Key Structure"))
  ;[1 0 0.01326] Deprecated - Old Fishing System
)

(event `ThrowLine`
  ;[1 0 0.01326] Deprecated - Old Fishing System
)

(event `ResetFishing`
  ;[1 0 0.01326] Deprecated - Old Fishing System
  (set `self.Deprecated_LineThrown` false)
  (set `self.Deprecated_BobberSpawned` false)
  (set `self.Deprecacted_BobberRef` null))

(event `Init_FishWidget`
  ;[1 0 0.01326] Deprecated - Old Fishing System
  (bind _returnvalue (`|CreateWidget` "/Game/Blueprints/J016221L/Proto_Widgets/W_CaughtFish.W_CaughtFish_C"))
  (`/Game/Blueprints/J016221L/Proto_Widgets/W_CaughtFish.Init_Widget` _returnvalue (`KismetTextLibrary.Conv_StringToText` "") (`KismetStringLibrary.Conv_DoubleToString` 0.0) null)
  (`UserWidget.AddToViewport` _returnvalue 0))

(event `SetWidgetVisibility`
  (params (`Visible?` :type Boolean))
  ;[1 0 0.01326] Deprecated - Old Fishing System
  ;;[1 1 1] Widget Visibility Toggle
)

(fn `UserConstructionScript`
  (`parent.UserConstructionScript`))