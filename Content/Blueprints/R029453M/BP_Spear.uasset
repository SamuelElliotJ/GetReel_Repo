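; BP_Spear is a thrown spear projectile for catching fish, which destroys itself on a timer after spawning.
; Launcher solves a toss velocity from origin to target, prints a miss if none is found, and activates projectile movement either way.
; The first fish overlapping its sphere is stored and reported to the player through FishCaught.
; A separate event builds the caught-fish widget from that fish's data, though its call here is unconnected.
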(event `self.ReceiveBeginPlay`
  (`KismetSystemLibrary.K2_SetTimerDelegate` (delegate `destroy`) 7.0))

(event `destroy`
  (`self.K2_DestroyActor`))

(event `Launcher`
  (params (Origin :type "Vector Structure") (Target :type "Vector Structure"))
  (bind _projectilemovement (`self.ProjectileMovement`))
  ;[1 1 1] throwing to picked point
  (bind (_tossvelocity _returnvalue) (`GameplayStatics.BlueprintSuggestProjectileVelocity` Origin Target 2500.0 0.0 "DoNotTrace"))
  (if _returnvalue
    (set `MovementComponent.Velocity` _tossvelocity _projectilemovement)
    (else
      (`KismetSystemLibrary.PrintString` "miss")))
  (`ActorComponent.Activate` _projectilemovement false))

(event `self.Sphere.OnComponentBeginOverlap`
  (params (OverlappedComponent :type "PrimitiveComponent Object Reference") (OtherActor :type "Actor Object Reference") (OtherComp :type "PrimitiveComponent Object Reference") (OtherBodyIndex :type Integer) (bFromSweep :type Boolean) (SweepResult :type "HitResult Structure (by ref)"))
  ;[1 1 1] hit fish?
  (bind _asai_fish (cast `/Game/Blueprints/Game/Fish/AI_Fish` OtherActor))
  (`/Engine/EditorBlueprintResources/StandardMacros.DoOnce` false
    (:`Completed`
      (bind _output_get (set `self.As BP Fish` _asai_fish))
      (`/Game/Blueprints/Characters/BP_Base_Character.FishCaught` (`self.PlayerRef`) _output_get self))))

(event `Init_FishWidget`
  (bind _data (`/Game/Blueprints/Game/Fish/AI_Fish.Data` (`self.As BP Fish`)))
  ;[1 1 1] show fish you catch
  (bind _returnvalue (`|CreateWidget` "/Game/Blueprints/J016221L/Proto_Widgets/W_CaughtFish.W_CaughtFish_C"))
  (`/Game/Blueprints/J016221L/Proto_Widgets/W_CaughtFish.Init_Widget` _returnvalue (`KismetTextLibrary.Conv_StringToText` (`DataAsset_Fish.AssetName` _data)) (`KismetStringLibrary.Conv_DoubleToString` (`DataAsset_Fish.AssetValue` _data)) (`DataAsset_Fish.AssetImage` _data))
  (`UserWidget.AddToViewport` _returnvalue 0))

(fn `UserConstructionScript`)