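; FeverTimeManager is an unfinished manager for a Fever Time bonus meant to start when a legendary fish is caught.
; BeginPlay only prints a not-working warning and shows the fever effect widget for five seconds.
; CaughtFishType checks rarity and cooldown before calling FeverTime, but FeverTime and CoolDown are empty.
; Their timer, GameMode flag and widget logic is disconnected, as is the fish-caught binding, leaving only Reset to clear the cooldown.
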(event `self.ReceiveBeginPlay`
  (`KismetSystemLibrary.PrintString` "Warning: FeverTime Not Working" true true (struct :`R` 1.0 :`A` 1.0) 60.0)
  (bind _returnvalue (`|CreateWidget` "/Game/Blueprints/C022272L/WBP_FeverTimeEffect.WBP_FeverTimeEffect_C" (`GameplayStatics.GetPlayerController` 0)))
  (bind _output_get (set `self.FTWidget` _returnvalue))
  (`UserWidget.AddToViewport` _output_get 0)
  (`KismetSystemLibrary.Delay` 5.0)
  (`Widget.RemoveFromParent` (`self.FTWidget`))
  (`KismetSystemLibrary.PrintString` "Remove Widget"))

(fn `CaughtFishType`
  (params (CaughtActor :type "/Game/Blueprints/Game/Fish/AI_Fish_Base Object Reference"))
  (if (and (`|EnumEquality` (`DataAsset_Fish.AssetRarity` (`/Game/Blueprints/Game/Fish/AI_Fish_Base.Data` CaughtActor)) "RLegendary") (not (`self.InCD?`)))
    (`self.FeverTime` CaughtActor)))

(fn `CoolDown`)

(fn `FeverTime`
  (params (CaughtActor :type "Object Object Reference")))

(fn `Reset`
  (set `self.InCD?` false)
  (`KismetSystemLibrary.K2_ClearAndInvalidateTimerHandle` (`self.CoolDown_TH`)))

(fn `UserConstructionScript`)