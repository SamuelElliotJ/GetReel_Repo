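; Weather effect manager, still unfinished, that switches the weather particles attached to the player character.
; On BeginPlay or WeatherM_Init it caches a PostProcessVolume, whose settings VolumeEditor overwrites with a fresh settings struct.
; SetCurrentWeatherEffect swaps the player's WeatherParticles asset by weather type, with Fog reusing the rain particle and Fair Sky setting none.
; Weather calculation events are empty stubs, and the looping check timer and test call are disconnected.
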(event `CalculateWeather`
  ;[1 1 1] Other is working on this so no continue on here
)

(event `defineWeather`
  ;[1 1 1] Other is working on this so no continue on here
)

(event `self.ReceiveBeginPlay`
  (bind _returnvalue (`GameplayStatics.GetActorOfClass` "/Script/Engine.PostProcessVolume" :!label _label))
  (`/Engine/EditorBlueprintResources/StandardMacros.IsValid` _returnvalue
    (:`Is Valid`
      (set `self.VolumeRef` _returnvalue))
    (:`Is Not Valid`
      (`KismetSystemLibrary.PrintString` "Post Process Volume Not Found" true true (struct :`R` 1.0 :`B` 0.055137 :`A` 1.0) 5.0))))

(event `WeatherM_Init`
  (goto _label))

(event `SetCurrentWeatherEffect`
  (params (CurrentWeather :type "/Game/Blueprints/C022272L/E_WeatherList Enum" :default "NewEnumerator0"))
  (bind _weatherparticles (`/Game/Blueprints/Characters/BP_Base_Character.WeatherParticles` (cast `/Game/Blueprints/Characters/BP_Base_Character` (`GameplayStatics.GetPlayerCharacter` 0) :!pure true)))
  (switch `/Game/Blueprints/C022272L/E_WeatherList` CurrentWeather
    (:`NewEnumerator0`
      (`NiagaraComponent.SetAsset` _weatherparticles null false))
    (:`NewEnumerator1`
      (`NiagaraComponent.SetAsset` _weatherparticles "/Game/Blueprints/C022272L/WeatherParticle/RainParticle_WithCollision.RainParticle_WithCollision" true))
    (:`NewEnumerator7`
      (`NiagaraComponent.SetAsset` _weatherparticles "/Game/Blueprints/C022272L/WeatherParticle/RainParticle_WithCollision.RainParticle_WithCollision" true))))

(fn `UserConstructionScript`)

(fn `VolumeEditor`
  (set `PostProcessVolume.Settings` (make `PostProcessSettings`) (`self.VolumeRef`)))