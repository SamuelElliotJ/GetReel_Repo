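; Day/night manager that runs the in-game clock, updates the game HUD's time and signals when the day finishes.
; Start_Day starts a looping timer that advances a time counter, scaled by DaySpeed, until the end hour clears it.
; Two chained timelines can sweep the directional light and refresh the sky sphere, but Start_Day does not start them.
; Lighting intensity and start-time sun selection logic is disconnected or unfinished.
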(event `Get References`
  (bind _asgm_get_reel_game (cast `/Game/Blueprints/Core/Gamemodes/GM_GetReel_Game` (`GameplayStatics.GetGameMode`)))
  (set `self.GameModeRef` _asgm_get_reel_game))

(event `Start_Day`
  ;[1 1 1] Begin Play
  (`self.Get References`)
  (`KismetSystemLibrary.Delay` 0.2)
  (set `self.TimeF` (* (`self.StartTime`) 0.5))
  (`self.Event Clock`))

(event `Play`
  ;[1 1 1] Sun Rotation
  (bind (_direction _alpha) (`Timeline|Timeline` :`NewTime` (* (stale `Event_StartTime_Morning` NewTime) 60.0) :!label _label)
    (:`Update`
      (`self.K2_SetActorRotation` (`self.DirectionLight`) (`KismetMathLibrary.MakeRotator` 0.0 (`KismetMathLibrary.Lerp` 90.0 -90.0 _alpha)) false)
      (`/Engine/EngineSky/BP_Sky_Sphere.UpdateSunDirection` (`self.SkySphereRef`)))
    (:`Finished`
      (`self.ReverseFromStart`))))

(event `Play_FromStart`
  ;[1 1 1] Sun Rotation
  (goto _label :!via `PlayFromStart`))

(event `Event_StartTime_Morning`
  (params (NewTime :type "Float (single-precision)"))
  ;[1 1 1] Sun Rotation
)

(event `StopClock`
  ;[1 1 1] Sun Rotation
  (`self.DayFinished`))

(event `Reverse`
  ;[1 1 1] Sun Rotation
  (bind (_direction _alpha) (`Timeline|Timeline_0` :`NewTime` (* (stale `Event_StartTimer_Evening` NewTime) 60.0) :!label _label_2) ; Issue was not changing the timeline length, thought using last keyframe would do it
    (:`Update`
      (`self.K2_SetActorRotation` (`self.DirectionLight`) (`KismetMathLibrary.MakeRotator` 0.0 (`KismetMathLibrary.Lerp` -90.0 -270.0 _alpha)) false)
      (`/Engine/EngineSky/BP_Sky_Sphere.UpdateSunDirection` (`self.SkySphereRef`)))
    (:`Finished`
      (`self.Play_FromStart`))))

(event `ReverseFromStart`
  ;[1 1 1] Sun Rotation
  (goto _label_2 :!via `PlayFromStart`))

(event `Event_StartTimer_Evening`
  (params (NewTime :type "Float (single-precision)"))
  ;[1 1 1] Sun Rotation
  (goto _label_2 :!via `SetNewTime`))

(event `Event Clock`
  ;[1 1 1] Clock
  (`self.IncrementClock`)
  (bind _returnvalue (`KismetSystemLibrary.K2_SetTimerDelegate` (delegate `IncrementClock`) 20.0 true))
  (set `self.ClockHandle` _returnvalue))

(event `IncrementClock`
  ;[1 1 1] Clock
  (`self.Clock` (* (`self.TimeF`) (`self.Day speed`)))
  (set `self.TimeF` (+ (`self.TimeF`) 0.5)))

(fn `Clock`
  (params (Delta :type "Float (double-precision)"))
  (bind _output_get (set `self.Time` (`KismetMathLibrary.MakeTimespan` 0 0 0 (`KismetMathLibrary.FTrunc` Delta))))
  (bind (_days _hours _minutes) (`KismetMathLibrary.BreakTimespan` _output_get))
  (if (== _hours (`self.EndTime`))
    (`self.StopClock`)
    (`KismetSystemLibrary.K2_ClearAndInvalidateTimerHandle` (`self.ClockHandle`)))
  (`/Game/Blueprints/Widgets/SubWidgets/W_Placeholder_Game.Update_Time` (`/Game/Blueprints/Core/Gamemodes/GM_GetReel_Game.GameHUD` (`self.GameModeRef`)) (`KismetTextLibrary.Conv_StringToText` (`KismetStringLibrary.Concat_StrStr` (`KismetTextLibrary.Conv_TextToString` (`KismetTextLibrary.Conv_DoubleToText` (`KismetMathLibrary.Conv_IntToDouble` _hours) "HalfToEven" false true 2)) ":" (`KismetTextLibrary.Conv_TextToString` (`KismetTextLibrary.Conv_DoubleToText` (`KismetMathLibrary.Conv_IntToDouble` _minutes) "HalfToEven" false true 2))))))

(fn `Day Lighting`
  (params (Delta :type "Float (double-precision)")))

(fn `Night Lighting`
  (params (Intensity :type "Float (double-precision)"))
  (`SkyLightComponent.SetIntensity` (`SkyLight.LightComponent` (`self.Skylight`)) Intensity))

(fn `UserConstructionScript`)