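; BP_Weather randomly picks the weather once initialised with a player reference, switching on that player's particle components for rain, lightning, wind, fog or snow.
; A nested weighted roll allows combinations such as foggy rain or windy storms, and can also leave the weather clear.
; Rain, wind, snow and thunder use 2D sounds created at BeginPlay, and lightning starts a looping timer with a randomised interval.
; StopWeather is marked deprecated.
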(event `self.ReceiveBeginPlay`
  (bind _returnvalue (`GameplayStatics.CreateSound2D` "/Game/Blueprints/BGM_SE/EnvironmentalSound/MS_RainOnly.MS_RainOnly" 1.0 1.0 0.0 null))
  (set `self.RainS` _returnvalue)
  (bind _returnvalue_2 (`GameplayStatics.CreateSound2D` "/Game/Blueprints/BGM_SE/EnvironmentalSound/MS_Windy.MS_Windy" 1.0 1.0 0.0 null))
  (set `self.WindS` _returnvalue_2)
  (bind _returnvalue_3 (`GameplayStatics.CreateSound2D` "/Game/Blueprints/BGM_SE/EnvironmentalSound/MS_Snowy.MS_Snowy" 1.0 1.0 0.0 null))
  (set `self.SnowS` _returnvalue_3)
  (bind _returnvalue_4 (`GameplayStatics.CreateSound2D` "/Game/Blueprints/BGM_SE/EnvironmentalSound/MS_Thunder3.MS_Thunder3" 1.0 1.0 0.0 null))
  (set `self.ThunderS` _returnvalue_4))

(event `Roll weather`
  ;[1 1 1] Roll
  (if (`KismetMathLibrary.RandomBoolWithWeight` 0.1)
    (`self.Start Rain`)
    (if (`KismetMathLibrary.RandomBoolWithWeight` 0.2)
      (`self.Start Lightning`)
      (if (`KismetMathLibrary.RandomBoolWithWeight` 0.5)
        (`self.Start Wind`)))
    (elif (`KismetMathLibrary.RandomBoolWithWeight` 0.1)
      (`self.Start Fog`)
      (if (`KismetMathLibrary.RandomBoolWithWeight` 0.3)
        (`self.Start Rain`)
        (if (`KismetMathLibrary.RandomBoolWithWeight` 0.2)
          (`self.Start Lightning`)))
      (elif (`KismetMathLibrary.RandomBoolWithWeight` 0.2)
        (`self.Start Wind`)
        (elif (`KismetMathLibrary.RandomBoolWithWeight` 0.1)
          (`self.Start Snow`))))))

(event `Initilaise`
  (params (`Player Ref` :type "/Game/Blueprints/Characters/BP_Base_Character Object Reference"))
  ;[1 1 1] Initialise
  (set `self.Player Ref` `Player Ref`)
  (`self.Roll weather`))

(event `Start Wind`
  ;[1 1 1] Wind
  (`ActorComponent.SetActive` (`/Game/Blueprints/Characters/BP_Base_Character.WeatherParticleWind` (`self.Player Ref`)) true false)
  (`AudioComponent.Play` (`self.WindS`) 0.0))

(event `Stop Weather`
  ;[1 1 1] Deprecated
  (`KismetSystemLibrary.K2_ClearAndInvalidateTimerHandle` (`self.Timer`))
  (`NiagaraComponent.SetAsset` (`/Game/Blueprints/Characters/BP_Base_Character.WeatherParticleSnow` (`self.Player Ref`)) null true)
  (`self.Stop All Sound`))

(event `Start Rain`
  ;[1 1 1] Rain
  (set `self.IsRaining` true)
  (`ActorComponent.SetActive` (`/Game/Blueprints/Characters/BP_Base_Character.WeatherParticleRain` (`self.Player Ref`)) true false)
  (`AudioComponent.Play` (`self.RainS`) 0.0))

(event `Start Lightning`
  (bind _player_ref (`self.Player Ref`))
  ;[1 1 1] Lightning
  (`ActorComponent.SetActive` (`/Game/Blueprints/Characters/BP_Base_Character.WeatherParticleLightning` _player_ref) true false)
  (`ActorComponent.SetActive` (`/Game/Blueprints/Characters/BP_Base_Character.WeatherParticleRain` _player_ref) true false)
  ;[1 1 1] ThumderSound
  (bind _returnvalue (`KismetSystemLibrary.K2_SetTimerDelegate` (`|CreateDelegate` :!event `PlayThunderSound`) (`KismetMathLibrary.RandomFloatInRange` 3.0 6.0) true))
  (set `self.ThunderTimerH` _returnvalue))

(event `Start WeatherEvent`
  ;[1 1 1] Deprecated
  (switch `int` (`KismetMathLibrary.RandomIntegerInRange` 0 2)
    (:`0`
      (`self.Start Rain`))
    (:`1`
      (`self.Start Snow`))
    (:`2`
      (`self.Start Fog`))))

(event `Start Snow`
  ;[1 1 1] Snow
  (if (not (`self.IsRaining`))
    (`ActorComponent.SetActive` (`/Game/Blueprints/Characters/BP_Base_Character.WeatherParticleSnow` (`self.Player Ref`)) true false)
    (`AudioComponent.Play` (`self.SnowS`) 0.0)))

(event `Start Fog`
  ;[1 1 1] Fog
  (`ActorComponent.SetActive` (`/Game/Blueprints/Characters/BP_Base_Character.WeatherParticleFog` (`self.Player Ref`)) true false))

(fn `PlayThunderSound`
  (`AudioComponent.Play` (`self.ThunderS`) 0.0))

(fn `Stop All Sound`
  (`AudioComponent.Stop` (`self.RainS`))
  (`AudioComponent.Stop` (`self.WindS`))
  (`AudioComponent.Stop` (`self.SnowS`))
  (`AudioComponent.Stop` (`self.ThunderS`))
  (`KismetSystemLibrary.K2_ClearAndInvalidateTimerHandle` (`self.ThunderTimerH`)))

(fn `UserConstructionScript`)