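; Day/night cycle Blueprint that rotates a directional light, refreshes the sky sphere and runs an in-game clock.
; Two chained timelines, morning and evening, each sweep the sun's pitch through half a turn, with StartTime choosing the first.
; A one-second looping timer advances a DaySpeed-scaled clock, prints it and stops at EndTime.
; Day/night light intensity switching is unfinished and disconnected.
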(event `self.ReceiveBeginPlay`
  ;[1 1 1] Begin Play
  (set `self.TimeF` (* (`self.StartTime`) 0.5))
  (if (> (`self.StartTime`) 12.0)
    (`self.Event_StartTimer_Evening` (- (`self.StartTime`) 12.0))
    (`self.Reverse`)
    (else
      (`self.Event_StartTime_Morning` (`self.StartTime`))
      (`self.Play`)))
  (`self.Event Clock`))

(event `Play`
  ;[1 1 1] Sun Rotation
  (bind (_direction _alpha) (`Timeline|Timeline` :`NewTime` (stale `Event_StartTime_Morning` NewTime) :!label _label)
    (:`Update`
      (`self.K2_SetActorRotation` (`self.DirectionLight`) (`KismetMathLibrary.MakeRotator` 0.0 (`KismetMathLibrary.Lerp` 90.0 -90.0 _alpha)) false)
      (`/Engine/EngineSky/BP_Sky_Sphere.UpdateSunDirection` (`self.SkySphereRef`)))
    (:`Finished`
      (`self.ReverseFromStart`))))

(event `Play_FromStart`
  ;[1 1 1] Sun Rotation
  (goto _label :!via `PlayFromStart`))

(event `Event_StartTime_Morning`
  (params (NewTime :type "Float (single-precision)"))
  ;[1 1 1] Sun Rotation
  (goto _label :!via `SetNewTime`))

(event `StopClock`
  ;[1 1 1] Sun Rotation
  (`|ExecutionSequence`
    (:`then_0`
      (goto _label :!via `Stop`))
    (:`then_1`
      (bind (_direction _alpha) (`Timeline|Timeline_0` :`NewTime` (stale `Event_StartTimer_Evening` NewTime) :!via `Stop` :!label _label_2)
        (:`Update`
          (`self.K2_SetActorRotation` (`self.DirectionLight`) (`KismetMathLibrary.MakeRotator` 0.0 (`KismetMathLibrary.Lerp` -90.0 -270.0 _alpha)) false)
          (`/Engine/EngineSky/BP_Sky_Sphere.UpdateSunDirection` (`self.SkySphereRef`)))
        (:`Finished`
          (`self.Play_FromStart`))))))

(event `Reverse`
  ;[1 1 1] Sun Rotation
  (goto _label_2))

(event `ReverseFromStart`
  ;[1 1 1] Sun Rotation
  (goto _label_2 :!via `PlayFromStart`))

(event `Event_StartTimer_Evening`
  (params (NewTime :type "Float (single-precision)"))
  ;[1 1 1] Sun Rotation
  (goto _label_2 :!via `SetNewTime`))

(event `Event Clock`
  ;[1 1 1] Clock
  (`self.IncrementClock`)
  (bind _returnvalue (`KismetSystemLibrary.K2_SetTimerDelegate` (delegate `IncrementClock`) 1.0 true))
  (set `self.ClockHandle` _returnvalue))

(event `IncrementClock`
  ;[1 1 1] Clock
  (`self.Clock` (* (`self.TimeF`) (`self.Day speed`)))
  (set `self.TimeF` (+ (`self.TimeF`) 0.5)))

(fn `Clock`
  (params (Delta :type "Float (double-precision)"))
  (bind _output_get (set `self.Time` (`KismetMathLibrary.MakeTimespan` 0 0 0 (`KismetMathLibrary.FTrunc` Delta))))
  (bind (_days _hours _minutes) (`KismetMathLibrary.BreakTimespan` _output_get))
  (if (== _hours (`self.EndTime`))
    (`self.StopClock`)
    (`KismetSystemLibrary.K2_ClearAndInvalidateTimerHandle` (`self.ClockHandle`)))
  (`KismetSystemLibrary.PrintString` (`KismetStringLibrary.Concat_StrStr` (`KismetTextLibrary.Conv_TextToString` (`KismetTextLibrary.Conv_DoubleToText` (`KismetMathLibrary.Conv_IntToDouble` _hours) "HalfToEven" false true 2)) ":" (`KismetTextLibrary.Conv_TextToString` (`KismetTextLibrary.Conv_DoubleToText` (`KismetMathLibrary.Conv_IntToDouble` _minutes) "HalfToEven" false true 2))) true true (struct :`G` 0.66 :`B` 1.0 :`A` 1.0) 10.0 "Time"))

(fn `Day Lighting`
  (params (Delta :type "Float (double-precision)")))

(fn `Night Lighting`
  (params (Intensity :type "Float (double-precision)"))
  (`SkyLightComponent.SetIntensity` (`SkyLight.LightComponent` (`self.Skylight`)) Intensity))

(fn `UserConstructionScript`)