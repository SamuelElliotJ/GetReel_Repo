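; BP_Throw_Hook is the physics-driven fishing hook projectile thrown from a fishing rod.
; InitHook stores the rod actor, attaches the cable's end to the rod mesh's HookSocket and launches the hook mesh with a fixed forward-and-up velocity-change impulse.
; The hit event is empty, and the logic to replace this actor with a BP_Hook linked to the rod is disconnected, so it never runs.
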(event `self.ReceiveBeginPlay`
  ;[1 1 1] Handle Launching Physics Hook
  (`KismetSystemLibrary.PrintString` "Throw Hook Spawned"))

(event `Init Hook`
  (params (`Actor Ref` :type "/Game/J016221L/Blueprint/BP_FishingRod Object Reference"))
  ;[1 1 1] Handle Launching Physics Hook
  (set `self.Actor Ref` `Actor Ref`)
  (`CableComponent.SetAttachEndToComponent` (`self.Cable`) (`/Game/J016221L/Blueprint/BP_FishingRod.SM_FishingRod` `Actor Ref`) "HookSocket")
  (`self.Launch Hook`))

(event `Launch Hook`
  ;[1 1 1] Handle Launching Physics Hook
  (`PrimitiveComponent.AddImpulse` (`self.SM_Hook`) (750.0 0.0 250.0) "None" true))

(event `self.SM_Hook.OnComponentHit`
  (params (HitComponent :type "PrimitiveComponent Object Reference") (OtherActor :type "Actor Object Reference") (OtherComp :type "PrimitiveComponent Object Reference") (NormalImpulse :type "Vector Structure") (Hit :type "HitResult Structure (by ref)")))

(fn `UserConstructionScript`)