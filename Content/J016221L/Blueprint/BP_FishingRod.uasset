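; BP_FishingRod is a fishing rod actor that toggles between casting and a catch attempt each time the player's action input fires.
; Casting plays a montage on the player mesh, and its notify spawns BP_Throw_Hook at the hook socket, initializes it with the rod, and hides the rod's hook and cable.
; The catch step is a stub that only prints a debug message.
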(event `self.ReceiveBeginPlay`
  ;[1 1 1] Bind Events On Begin Play
  (add `/Game/TopDown/Blueprints/BP_Base_Character.ActionPressed` (`self.PlayerRef`) (`|CreateDelegate` :!event `ActionPressed`)))

(event `ActionPressed`
  ;[1 1 1] Handle Fishing Mechanics
  (if (`self.ActionPressed?`)
    (`self.CatchFish`)
    (set `self.ActionPressed?` false)
    (else
      (`self.ThrowLine`)
      (set `self.ActionPressed?` true))))

(event `ThrowLine`
  ;[1 1 1] Handle Fishing Mechanics
  (`KismetSystemLibrary.PrintString` "Throw Line")
  (bind _notifyname (`|PlayMontage` (`Character.Mesh` (`self.PlayerRef`)) "/Game/J016221L/Proto_Character/Proto_Animation/Fishing_Cast_Montage.Fishing_Cast_Montage")
    (:`OnNotifyBegin`
      (`KismetSystemLibrary.PrintString` (`KismetStringLibrary.Conv_NameToString` _notifyname))
      (bind _returnvalue (`|SpawnActorFromClass` "/Game/J016221L/Blueprint/BP_Throw_Hook.BP_Throw_Hook_C" (`SceneComponent.GetSocketTransform` (`self.SM_Hook`) "HookSocket" "RTS_World") "Undefined" "MultiplyWithRoot" null null null))
      (`/Game/J016221L/Blueprint/BP_Throw_Hook.Init Hook` _returnvalue self)
      (`SceneComponent.SetHiddenInGame` (`self.SM_Hook`) true false)
      (`SceneComponent.SetHiddenInGame` (`self.Cable`) true false))))

(event `CatchFish`
  ;[1 1 1] Handle Fishing Mechanics
  (`KismetSystemLibrary.PrintString` "Attempt to Catch Fish"))

(fn `UserConstructionScript`)