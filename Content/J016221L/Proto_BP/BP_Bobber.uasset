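; Fishing bobber actor that attaches a cable to a given actor, bobs in the water and gets reeled in.
; A looping timer and timeline dip it, stopping at a bob count of three to show a widget.
; Reeling at another count destroys the fish as "Got Away".
; A timeline sweeps it horizontally to the end location, opens the player's fish widget if the fish remains, then resets fishing and destroys itself.
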(event `StartReel`
  (params (EndLocation :type "Vector Structure") (PlayerRef :type "/Game/TopDown/Blueprints/BP_ProtoCharacter_2 Object Reference"))
  (bind (_initloc_x _initloc_y _initloc_z) (`KismetMathLibrary.BreakVector` (`self.InitLoc`)))
  (if (== (`self.BobCount`) 3)
    (bind (_direction _alpha) (`Timeline|Reel_Timeline` :!label _label)
      (:`Update`
        (`self.K2_SetActorLocation` (`KismetMathLibrary.VLerp` (`KismetMathLibrary.MakeVector` _initloc_x _initloc_y _initloc_z) (`KismetMathLibrary.MakeVector` EndLocation_X EndLocation_Y _initloc_z) _alpha) true))
      (:`Finished`
        (bind _fishref (`self.FishRef`)
          (:`then`
            (`/Game/TopDown/Blueprints/BP_ProtoCharacter_2.Init_FishWidget` PlayerRef)
            (`self.K2_DestroyActor` _fishref))
          (:`else`
            _))
        (`/Game/TopDown/Blueprints/BP_ProtoCharacter_2.ResetFishing` PlayerRef)
        (`self.K2_DestroyActor`)))
    (else
      (`self.StopBobbing`)
      (`KismetSystemLibrary.PrintString` "Fish Got Away")
      (`self.K2_DestroyActor` (`self.FishRef`))
      (goto _label))))

(event `StopReel`
  (goto _label :!via `Stop`))

(event `Init`
  (params (Actor :type "Actor Object Reference"))
  (set `self.BobCount` 0)
  (`CableComponent.SetAttachEndTo` (`self.Cable`) Actor "None" "None")
  (set `self.InitLoc` (`self.K2_GetActorLocation`)))

(event `StopBobbing`
  (`KismetSystemLibrary.K2_ClearAndInvalidateTimerHandle` (`self.BobTimer`)))

(event `StartBobbing`
  (`/Engine/EditorBlueprintResources/StandardMacros.DoOnce` false
    (:`Completed`
      (set `self.InitLoc` (`self.K2_GetActorLocation`))
      (`self.Bob`)
      (bind _returnvalue (`KismetSystemLibrary.K2_SetTimerDelegate` (`|CreateDelegate` :!event `Bob`) 1.0 true))
      (set `self.BobTimer` _returnvalue))))

(event `Bob`
  (bind _initloc (`self.InitLoc`))
  (bind (_direction _alpha) (`Timeline|Timeline_Bob` :!via `PlayFromStart`)
    (:`Update`
      (`self.K2_SetActorLocation` (`KismetMathLibrary.VLerp` _initloc (- _initloc (0.0 0.0 20.0)) _alpha)))
    (:`Finished`
      (bind _result (`/Engine/EditorBlueprintResources/StandardMacros.IncrementInt` (`self.BobCount`))
        (:`  `
          (switch `int` _result
            (:`3`
              (`self.StopBobbing`)
              (`self.SetWidgetVisibility` true))))))))

(event `SetWidgetVisibility`
  (params (`Visible?` :type Boolean))
  (`SceneComponent.SetHiddenInGame` (`self.Widget`) (not `Visible?`) false))

(fn `UserConstructionScript`)