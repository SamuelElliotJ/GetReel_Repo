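; BP_Bobber_Throwable is the thrown form of a bobber, trailing a cable to the player who launched it.
; Launch applies a fixed impulse to the sphere, mostly along +X, attaches the cable's end to the given actor and stores that actor.
; On the sphere's first hit it spawns and initializes a BP_Bobber there, reports it to BP_ProtoCharacter_2, then destroys itself.
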(event `Launch`
  (params (Actor :type "Actor Object Reference"))
  (`PrimitiveComponent.AddImpulse` (`self.Sphere`) (30000.0 0.0 250.0) "None" false)
  (`CableComponent.SetAttachEndTo` (`self.Cable`) Actor "None" "None")
  (set `self.PlayerRef` Actor))

(event `self.Sphere.OnComponentHit`
  (params (HitComponent :type "PrimitiveComponent Object Reference") (OtherActor :type "Actor Object Reference") (OtherComp :type "PrimitiveComponent Object Reference") (NormalImpulse :type "Vector Structure") (Hit :type "HitResult Structure (by ref)"))
  (bind _playerref (`self.PlayerRef`))
  (bind _returnvalue (`|SpawnActorFromClass` "/Game/J016221L/Proto_BP/BP_Bobber.BP_Bobber_C" (`KismetMathLibrary.MakeTransform` (`SceneComponent.K2_GetComponentLocation` (`self.Sphere`))) "Undefined" "MultiplyWithRoot" null null))
  (`/Game/J016221L/Proto_BP/BP_Bobber.Init` _returnvalue _playerref)
  (bind _asbp_proto_character_2 (cast `/Game/TopDown/Blueprints/BP_ProtoCharacter_2` _playerref))
  (`/Game/TopDown/Blueprints/BP_ProtoCharacter_2.SetBobberSpawned` _asbp_proto_character_2 _returnvalue true)
  (`self.K2_DestroyActor`))

(fn `UserConstructionScript`)