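; BP_BasicFish is an AI fish for fishing that wanders around and is drawn to a nearby bobber.
; It loops AIMoveTo toward random reachable points while it has no valid target.
; A timer-driven sphere trace finds a BP_Bobber, registers the fish on it and steers there at the fish's own height.
; Arrival triggers StartBobbing once; wandering resumes and that latch resets when the reached bobber becomes invalid.
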(event `self.ReceiveBeginPlay`
  (`self.RunAi`)
  (bind _returnvalue (`KismetSystemLibrary.K2_SetTimerDelegate` (delegate `Search`) 0.1 true))
  (set `self.SearchHandle` _returnvalue)
  (set `self.Target` null))

(event `Search`
  (bind _returnvalue (`self.K2_GetActorLocation`))
  (bind (_returnvalue_x _returnvalue_y _returnvalue_z) (`KismetMathLibrary.BreakVector` (`self.K2_GetActorLocation`)))
  (bind _target (`self.Target`))
  (bind (_returnvalue_x_2 _returnvalue_y_2) (`KismetMathLibrary.BreakVector` (`self.K2_GetActorLocation` (`self.Target`))))
  (bind (_outhits _returnvalue_2) (`KismetSystemLibrary.SphereTraceMultiForObjects` _returnvalue _returnvalue 200.0 (`|MakeArray` "ObjectTypeQuery1" "ObjectTypeQuery2" "ObjectTypeQuery3" :!type "EObjectTypeQuery Enum")))
  (if _returnvalue_2
    (for _array_element _outhits
      (bind _asbp_bobber (cast `/Game/J016221L/Proto_BP/BP_Bobber` (`.HitActor` (`GameplayStatics.BreakHitResult` _array_element))))
      (bind _output_get (set `self.Target` _asbp_bobber))
      (set `/Game/J016221L/Proto_BP/BP_Bobber.FishRef` self _output_get)
      (break))
    (`self.Target`
      (:`then`
        (`|AIMoveTo` self (`KismetMathLibrary.MakeVector` _returnvalue_x_2 _returnvalue_y_2 _returnvalue_z) null 0.0 true
          (:`OnSuccess`
            (set `self.TargetFound?` true)
            (`/Engine/EditorBlueprintResources/StandardMacros.DoOnce` false :!label _label
              (:`Completed`
                (`/Engine/EditorBlueprintResources/StandardMacros.IsValid` _target
                  (:`Is Valid`
                    (`/Game/J016221L/Proto_BP/BP_Bobber.StartBobbing` _target))))))))
      (:`else`
        (if (`self.TargetFound?`)
          (set `self.TargetFound?` false)
          (`self.RunAi`)
          (goto _label :!via `Reset`))))))

(event `RunAi`
  (`self.Target`
    (:`then`)
    (:`else`
      (bind _returnvalue (`self.GetMoveToLocation`))
      (`self.Move` _returnvalue))))

(event `Move`
  (params (Destination :type "Vector Structure"))
  (`|AIMoveTo` self Destination null 0.0 true
    (:`OnSuccess`
      (`KismetSystemLibrary.Delay` 0.2)
      (`self.RunAi`))
    (:`OnFail`
      (`self.RunAi`))))

(fn `GetMoveToLocation`
  (returns (ReturnValue :type "Vector Structure"))
  (bind _randomlocation (`NavigationSystemV1.K2_GetRandomReachablePointInRadius` (`self.K2_GetActorLocation`) 500.0 null null))
  (if (`AIBlueprintHelperLibrary.IsValidAILocation` _randomlocation)
    (return _randomlocation)
    (else
      (`self.RunAi`))))

(fn `UserConstructionScript`)